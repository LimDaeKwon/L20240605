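; BP_Actor is an Actor that slides its Sphere component back and forth along its relative X axis.
; Each Tick steps XPosition one unit in the IsRight direction, applies it to the sphere and flips direction past either end of a fixed range.
; Movement is per frame rather than scaled by delta time, which is only printed for debugging.
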(event EventTick
  (params (DeltaSeconds :type Float%20%28single-precision%29))
  (Development|PrintString (Utilities|String|ToString(Float) DeltaSeconds))
  (if (Variables|Default|GetIsRight)
    (bind _output_get (Variables|Default|SetXPosition (+ (Variables|Default|GetXPosition) 1.0)))
    (Transformation|SetRelativeLocation (Variables|Default|GetSphere) (Math|Vector|MakeVector _output_get 0.0 0.0) false false)
    (if (> (Variables|Default|GetXPosition) 2e+02)
      (Variables|Default|SetIsRight false))
    (else
      (bind _output_get_2 (Variables|Default|SetXPosition (+ (Variables|Default|GetXPosition) -1.0)))
      (Transformation|SetRelativeLocation (Variables|Default|GetSphere) (Math|Vector|MakeVector _output_get_2 0.0 0.0) false false)
      (if (< (Variables|Default|GetXPosition) 0.0)
        (Variables|Default|SetIsRight true)))))

(fn ConstructionScript)