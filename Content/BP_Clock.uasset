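; BP_Clock is a clock that shows a running, accelerated time count on a TextRender component.
; Each Tick adds delta seconds scaled by 100 to a running total, then displays the total divided by 60 and its remainder, separated by a colon.
; The FloatToStr00 helper floors each value and zero-pads it to two digits; the left field never wraps.
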(event EventTick
  (params (DeltaSeconds :type Float%20%28single-precision%29))
  (bind _output_get (Variables|Default|SetTotalDeltaSeconds (+ (Variables|Default|GetTotalDeltaSeconds) (* DeltaSeconds 1e+02))))
  (Rendering|Components|TextRender|SetText (Variables|Default|GetTextRender) (Utilities|Text|ToText(String) (Utilities|String|Append (CallFunction|FloattoStr00 (/ _output_get 6e+01)) ":" (CallFunction|FloattoStr00 (Math|Float|%(Float) _output_get 6e+01))))))

(fn ConstructionScript)

(fn FloattoStr00
  (params (Number :type Float%20%28double-precision%29))
  (bind _returnvalue (Math|Float|Floor Number))
  (if (< Number 1e+01)
    (return (Utilities|String|Append "0" (Utilities|String|ToString(Integer) _returnvalue)))
    (else
      (return (Utilities|String|ToString(Integer) _returnvalue)))))