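; Actor that moves its Sphere component around a rectangular loop in its local XZ plane.
; Each Tick switches on the MoveType enum (Right, Up, Left, Down), steps X or Z by a fixed amount and sets the sphere's relative location.
; Crossing that side's limit advances MoveType to the next direction, forming a simple state machine.
; Movement is per frame without delta time, so speed depends on frame rate.
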(event EventTick
  (params (DeltaSeconds :type Float%20%28single-precision%29))
  (switch Utilities|FlowControl|Switch|SwitchonEN_MoveType (Variables|Default|GetMoveType)
    (:NewEnumerator0
      (bind _output_get (Variables|Default|SetXPosition (+ (Variables|Default|GetXPosition) 5.0)))
      (Transformation|SetRelativeLocation (Variables|Default|GetSphere) (Math|Vector|MakeVector _output_get 0.0 (Variables|Default|GetZPosition)) false false)
      (if (> (Variables|Default|GetXPosition) 2e+02)
        (Variables|Default|SetMoveType "NewEnumerator1")))
    (:NewEnumerator1
      (bind _output_get_2 (Variables|Default|SetZPosition (+ (Variables|Default|GetZPosition) 5.0)))
      (Transformation|SetRelativeLocation (Variables|Default|GetSphere) (Math|Vector|MakeVector (Variables|Default|GetXPosition) 0.0 _output_get_2) false false)
      (if (> (Variables|Default|GetZPosition) 2e+02)
        (Variables|Default|SetMoveType "NewEnumerator2")))
    (:NewEnumerator2
      (bind _output_get_3 (Variables|Default|SetXPosition (+ (Variables|Default|GetXPosition) -5.0)))
      (Transformation|SetRelativeLocation (Variables|Default|GetSphere) (Math|Vector|MakeVector _output_get_3 0.0 (Variables|Default|GetZPosition)) false false)
      (if (< (Variables|Default|GetXPosition) 0.0)
        (Variables|Default|SetMoveType "NewEnumerator3")))
    (:NewEnumerator3
      (bind _output_get_4 (Variables|Default|SetZPosition (+ (Variables|Default|GetZPosition) -5.0)))
      (Transformation|SetRelativeLocation (Variables|Default|GetSphere) (Math|Vector|MakeVector (Variables|Default|GetXPosition) 0.0 _output_get_4) false false)
      (if (< (Variables|Default|GetZPosition) 0.0)
        (Variables|Default|SetMoveType "NewEnumerator0")))))

(fn ConstructionScript)